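; BP_PlayerCharacter_2 is a player character Blueprint that toggles an aiming mode with the right mouse button.
; Holding the button sets IsAiming, makes the character turn toward controller rotation and raises its rotation rate for snappier turning.
; Releasing it clears the flag and restores slower rotation toward movement direction.
; BeginPlay and the construction script only call their parents, while overlap and Tick are disabled.
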(event `Key|RightMouseButton`
  (params (Key :type "Key Structure"))
  (bind _charactermovement (`self.CharacterMovement`))
  (:`Pressed`
    (set `self.IsAiming` true)
    (set `CharacterMovementComponent.bOrientRotationToMovement` false _charactermovement)
    (set `CharacterMovementComponent.bUseControllerDesiredRotation` true _charactermovement)
    (set `CharacterMovementComponent.RotationRate` (struct :`Yaw` 1100.0) _charactermovement))
  (:`Released`
    (set `self.IsAiming` false)
    (set `CharacterMovementComponent.bOrientRotationToMovement` true _charactermovement)
    (set `CharacterMovementComponent.bUseControllerDesiredRotation` false _charactermovement)
    (set `CharacterMovementComponent.RotationRate` (struct :`Yaw` 500.0) _charactermovement)))

(event `self.ReceiveBeginPlay`
  (`parent.ReceiveBeginPlay`))

(fn `UserConstructionScript`
  (`parent.UserConstructionScript`))