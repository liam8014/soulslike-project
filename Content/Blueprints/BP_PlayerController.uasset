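; Player controller that shows a focus indicator widget over the current focus target.
; BeginPlay creates the WBP_FocusIndicator widget, adds it to the viewport hidden and stores it.
; Each Tick, a valid CurrentFocusTarget makes it visible and moves it to the screen projection of a point slightly above that actor.
; Without a target it hides the widget and writes a debug log line; nothing here sets the target.
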(event `self.ReceiveBeginPlay`
  (bind _returnvalue (`|CreateWidget` "/Game/04_UI/WBP_FocusIndicator.WBP_FocusIndicator_C"))
  (`UserWidget.AddToViewport` _returnvalue 0)
  (`Widget.SetVisibility` _returnvalue "Hidden")
  (set `self.FocusIndicatorHUD` _returnvalue))

(event `self.ReceiveTick`
  (params (DeltaSeconds :type "Float (single-precision)"))
  (if (`KismetSystemLibrary.IsValid` (`self.CurrentFocusTarget`))
    (`Widget.SetVisibility` (stale `self.ReceiveBeginPlay` _returnvalue) "Visible")
    (`UserWidget.SetPositionInViewport` (`self.FocusIndicatorHUD`) (`WidgetLayoutLibrary.ProjectWorldLocationToWidgetPosition` self (+ (`self.K2_GetActorLocation` (`self.CurrentFocusTarget`)) (0.0 0.0 50.0))) true)
    (else
      (`Widget.SetVisibility` (stale `self.ReceiveBeginPlay` _returnvalue) "Hidden")
      (`KismetSystemLibrary.LogString` "false"))))

(fn `UserConstructionScript`)